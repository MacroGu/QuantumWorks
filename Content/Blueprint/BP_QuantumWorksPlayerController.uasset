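; Player controller that installs a Sobel outline post-process effect when play begins, using the stencil variant by default.
; SetOutlinePostProcessMaterial creates a transient dynamic instance of either the stencil or depth material, chosen by a boolean, and stores it as OutlineMid.
; It then sets that instance as the sole blendable on the first PostProcessVolume found, printing the selected mode or an error if no volume exists.
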(event `self.ReceiveBeginPlay`
  (`self.Set Outline Post Process Material` true))

(event `Key|LeftMouseButton`
  (params (Key :type "Key Structure")))

(fn `Set Outline Post Process Material`
  (params (UseStencilSobel :type Boolean))
  (`|ExecutionSequence`
    (:`then_0`
      (if UseStencilSobel
        (bind _returnvalue (`KismetMaterialLibrary.CreateDynamicMaterialInstance` (`self.OutlinePostProcessStencilMIC`) "Stencil" "Transient"))
        (set `self.OutlineMid` _returnvalue)
        (else
          (bind _returnvalue_2 (`KismetMaterialLibrary.CreateDynamicMaterialInstance` (`self.OutlinePostProcessDepthMIC`) "Depth" "Transient"))
          (set `self.OutlineMid` _returnvalue_2))))
    (:`then_1`
      (bind _outactors (`GameplayStatics.GetAllActorsOfClass` "/Script/Engine.PostProcessVolume"))
      (if (> (`KismetArrayLibrary.Array_Length` _outactors) 0)
        (setmembers `PostProcessSettings` :`StructRef` (`PostProcessVolume.Settings` (`|GetArrayItem` _outactors)) :`WeightedBlendables` (make `WeightedBlendables` (`|MakeArray` (make `WeightedBlendable` 1.0 (`self.OutlineMid`)))))
        (else
          (`KismetSystemLibrary.PrintString` "Post process volume not set correctly." true true (struct :`R` 1.0 :`A` 1.0)))))
    (:`then_2`
      (if UseStencilSobel
        (`KismetSystemLibrary.PrintString` "Switched to stencil sobel.")
        (else
          (`KismetSystemLibrary.PrintString` "Switched to depth sobel."))))))

(fn `UserConstructionScript`)